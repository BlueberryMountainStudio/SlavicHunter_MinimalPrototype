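; BP_Foe is a foe actor whose sphere changes material to show highlight, hover and selection feedback.
; Cursor over and out events track hover, showing red on a highlighted foe and restoring brown when the foe is not selected.
; Highlight and Dehighlight switch the state and material.
; Select marks the foe selected if hovered, otherwise clears an existing selection and restores the material for the current state.
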(event OnBeginCursorOver(Sphere)
  (params (TouchedComponent :type Primitive%20Component%20Object%20Reference))
  (Variables|Default|SetHovered? true)
  (if (Utilities|Enum|Equal(Enum) (Variables|Default|GetStates) "NewEnumerator1")
    (Rendering|Material|SetMaterial TouchedComponent 0 "/Game/Programming/GreyboxAssetsAndMaterials/HoveredRed.HoveredRed")))

(event OnEndCursorOver(Sphere)
  (params (TouchedComponent :type Primitive%20Component%20Object%20Reference))
  (Variables|Default|SetHovered? false)
  (if (not (Variables|Default|GetSelected?))
    (switch Utilities|FlowControl|Switch|SwitchonFoeStates (Variables|Default|GetStates)
      (:NewEnumerator0
        (Rendering|Material|SetMaterial TouchedComponent 0 "/Game/Programming/GreyboxAssetsAndMaterials/BasicBrown.BasicBrown"))
      (:NewEnumerator1
        (Rendering|Material|SetMaterial TouchedComponent 0 "/Game/Programming/GreyboxAssetsAndMaterials/HighlightBrown.HighlightBrown")))))

(event EventBeginPlay)

(event Collision|EventActorBeginOverlap
  (params (OtherActor :type Actor%20Object%20Reference)))

(event EventTick
  (params (DeltaSeconds :type Float%20%28single-precision%29)))

(fn ConstructionScript)

(fn Highlight
  (bind _sphere (Variables|Default|GetSphere))
  (Rendering|Material|SetMaterial _sphere 0 "/Game/Programming/GreyboxAssetsAndMaterials/HighlightBrown.HighlightBrown")
  (Variables|Default|SetStates "NewEnumerator1")
  (if (Variables|Default|GetHovered?)
    (Rendering|Material|SetMaterial _sphere 0 "/Game/Programming/GreyboxAssetsAndMaterials/HoveredRed.HoveredRed")))

(fn Dehighlight
  (Rendering|Material|SetMaterial (Variables|Default|GetSphere) 0 "/Game/Programming/GreyboxAssetsAndMaterials/BasicBrown.BasicBrown")
  (Variables|Default|SetStates "NewEnumerator0"))

(fn Select
  (if (Variables|Default|GetHovered?)
    (Variables|Default|SetSelected? true)
    (Rendering|Material|SetMaterial (Variables|Default|GetSphere) 0 "/Game/Programming/GreyboxAssetsAndMaterials/BasicRed.BasicRed")
    (return (Variables|Default|GetSelected?))
    (elif (Variables|Default|GetSelected?)
      (Variables|Default|SetSelected? false)
      (switch Utilities|FlowControl|Switch|SwitchonFoeStates (Variables|Default|GetStates)
        (:NewEnumerator0
          (Rendering|Material|SetMaterial (Variables|Default|GetSphere) 0 "/Game/Programming/GreyboxAssetsAndMaterials/BasicBrown.BasicBrown")
          (return (Variables|Default|GetSelected?)))
        (:NewEnumerator1
          (Rendering|Material|SetMaterial (Variables|Default|GetSphere) 0 "/Game/Programming/GreyboxAssetsAndMaterials/HighlightBrown.HighlightBrown")
          (return (Variables|Default|GetSelected?)))))))