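; BP_Foe is a huntable target actor with cursor-driven highlighting and selection, plus hit-location damage.
; Highlight, Dehighlight, Select and cursor events on the Hase component swap its material from the hover, highlight and selected states.
; TakeDamage scales damage by body-part multipliers; on death it adds the foe's class and hit location to the shooter's inventory, then destroys the actor.
; Surviving a hit calls Flee, which is currently an empty stub.
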(event OnBeginCursorOver(Hase)
  (params (TouchedComponent :type Primitive%20Component%20Object%20Reference))
  (Variables|Default|SetHovered? true)
  (if (Utilities|Enum|Equal(Enum) (Variables|Default|GetStates) "NewEnumerator1")
    (Rendering|Material|SetMaterial TouchedComponent 0 "/Game/Programming/GreyboxAssetsAndMaterials/HoveredRed.HoveredRed")))

(event OnEndCursorOver(Hase)
  (params (TouchedComponent :type Primitive%20Component%20Object%20Reference))
  (Variables|Default|SetHovered? false)
  (if (not (Variables|Default|GetSelected?))
    (switch Utilities|FlowControl|Switch|SwitchonFoeStates (Variables|Default|GetStates)
      (:NewEnumerator0
        (Rendering|Material|SetMaterial TouchedComponent 0 "/Game/Programming/GreyboxAssetsAndMaterials/BasicBrown.BasicBrown"))
      (:NewEnumerator1
        (Rendering|Material|SetMaterial TouchedComponent 0 "/Game/Programming/GreyboxAssetsAndMaterials/HighlightBrown.HighlightBrown")))))

(event EventBeginPlay)

(event Collision|EventActorBeginOverlap
  (params (OtherActor :type Actor%20Object%20Reference)))

(event EventTick
  (params (DeltaSeconds :type Float%20%28single-precision%29)))

(fn ConstructionScript)

(fn Highlight
  (bind _hase (Variables|Default|GetHase))
  (Rendering|Material|SetMaterial _hase 0 "/Game/Programming/GreyboxAssetsAndMaterials/HighlightBrown.HighlightBrown")
  (Variables|Default|SetStates "NewEnumerator1")
  (if (Variables|Default|GetHovered?)
    (Rendering|Material|SetMaterial _hase 0 "/Game/Programming/GreyboxAssetsAndMaterials/HoveredRed.HoveredRed")))

(fn Dehighlight
  (Rendering|Material|SetMaterial (Variables|Default|GetHase) 0 "/Game/Programming/GreyboxAssetsAndMaterials/BasicBrown.BasicBrown")
  (Variables|Default|SetStates "NewEnumerator0"))

(fn Select
  (if (Variables|Default|GetHovered?)
    (Variables|Default|SetSelected? true)
    (Rendering|Material|SetMaterial (Variables|Default|GetHase) 0 "/Game/Programming/GreyboxAssetsAndMaterials/BasicRed.BasicRed")
    (return (Variables|Default|GetSelected?))
    (elif (Variables|Default|GetSelected?)
      (Variables|Default|SetSelected? false)
      (switch Utilities|FlowControl|Switch|SwitchonFoeStates (Variables|Default|GetStates)
        (:NewEnumerator0
          (Rendering|Material|SetMaterial (Variables|Default|GetHase) 0 "/Game/Programming/GreyboxAssetsAndMaterials/BasicBrown.BasicBrown")
          (return (Variables|Default|GetSelected?)))
        (:NewEnumerator1
          (Rendering|Material|SetMaterial (Variables|Default|GetHase) 0 "/Game/Programming/GreyboxAssetsAndMaterials/HighlightBrown.HighlightBrown")
          (return (Variables|Default|GetSelected?)))))))

(fn TakeDamage
  (params (Damage :type Float%20%28double-precision%29) (HitAt :type HitZones%20Enum :default "NewEnumerator0") (ShootingPlayerREF :type BP%20Player%20Character%20Object%20Reference))
  (switch Utilities|FlowControl|Switch|SwitchonHitZones HitAt
    (:NewEnumerator0
      (Variables|GameDesign|SetHealth (- (Variables|GameDesign|GetHealth) Damage)))
    (:NewEnumerator1
      (Variables|GameDesign|SetHealth (- (Variables|GameDesign|GetHealth) (* Damage (Variables|GameDesign|GetWeakMultiplier)))))
    (:NewEnumerator2
      (Variables|GameDesign|SetHealth (- (Variables|GameDesign|GetHealth) (* Damage (Variables|GameDesign|GetLungMultiplier%20)))))
    (:NewEnumerator3
      (Variables|GameDesign|SetHealth (- (Variables|GameDesign|GetHealth) (* Damage (Variables|GameDesign|GetHeartMultiplier)))))
    (:NewEnumerator4
      (Variables|GameDesign|SetHealth (- (Variables|GameDesign|GetHealth) (* Damage (Variables|GameDesign|GetHeadMultiplier))))))
  (if (<= (Variables|GameDesign|GetHealth) 0.0)
    (Utilities|Array|Add (Variables|/Game/Programming/Blueprints/BP_PlayerCharacter.BP_PlayerCharacter_C|GetInventory ShootingPlayerREF) (Utilities|Struct|MakeInventoryStruct (Utilities|GetClass self) HitAt))
    (Actor|DestroyActor)
    (else
      (CallFunction|Flee))))

(fn Flee)