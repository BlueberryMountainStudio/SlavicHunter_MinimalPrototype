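; BP_Habitat is a spawner actor that populates a spherical area with foes of a configurable class when play begins.
; The construction script sizes the Container sphere from Radius.
; BeginPlay loops over a count derived from SpawnAmount, picking random points within the sphere's bounds and line-tracing from high above along inverted actor up against AttachtoObjects types.
; Hits spawn FoeToSpawn at the impact location, while misses loop back to trace again without a retry limit.
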(event EventBeginPlay
  (bind _container (Variables|Default|GetContainer))
  (bind (_origin _boxextent _sphereradius) (Collision|GetComponentBounds _container))
  (bind _result (Math|Integer|DecrementInt (Variables|GameDesign|GetSpawnAmount))
    (:%20%20
      (switch Utilities|FlowControl|Switch|SwitchonSpawnBehaviours (Variables|GameDesign|GetSpawn%20Behaviours)
        (:NewEnumerator0
          (for _index (range 0 _result)
            (bind (_x _y) (CallFunction|GetRandomPointinCircle _origin _sphereradius))
            (bind (_outhit _returnvalue) (Collision|LineTraceForObjects (Math|Vector|MakeVector _x _y (+ 0.0 1e+05)) (+ (Math|Vector|MakeVector _x _y (+ 0.0 1e+05)) (* (* (Transformation|GetActorUpVector) -1) 1.5e+05)) (Variables|GameDesign|GetAttachtoObjects) false 0 "None" :!label _label))
            (if _returnvalue
              (Game|SpawnActorfromClass (Variables|GameDesign|GetFoeToSpawn) (Math|Transform|MakeTransform (.Location (Collision|BreakHitResult _outhit)) "0, 0, 0" "1.000000,1.000000,1.000000") "Undefined" "MultiplyWithRoot" 0 0)
              (else
                (goto _label)))))))))

(fn ConstructionScript
  (Components|Sphere|SetSphereRadius (Variables|Default|GetContainer) (Variables|GameDesign|GetRadius) false))