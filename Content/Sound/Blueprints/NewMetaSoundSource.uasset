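; Test actor that plays a MetaSound-style instrument on its Audio component from four keyboard keys.
; BeginPlay enables input from player controller 0 so the actor receives the key presses.
; Each key sets the "MIDI In" float to a fixed note, spaced in major thirds from middle C, then fires the shared "Trigger" parameter.
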(event EventBeginPlay
  (Input|EnableInput (Game|GetPlayerController 0)))

(event Collision|EventActorBeginOverlap
  (params (OtherActor :type Actor%20Object%20Reference)))

(event EventTick
  (params (DeltaSeconds :type Float%20%28single-precision%29)))

(event Input|KeyboardEvents|Hyphen
  (params (Key :type Key%20Structure :default "None"))
  (bind _audio (Variables|Default|GetAudio))
  (:Pressed
    (Audio|Parameter|SetFloatParameter _audio "MIDI In" 72.0 :!class /Script/AudioExtensions.AudioParameterControllerInterface)
    (Class|AudioParameterControllerInterface|SetTriggerParameter _audio "Trigger")))

(event Input|KeyboardEvents|Ö
  (params (Key :type Key%20Structure :default "None"))
  (bind _audio (Variables|Default|GetAudio))
  (:Pressed
    (Audio|Parameter|SetFloatParameter _audio "MIDI In" 6e+01 :!class /Script/AudioExtensions.AudioParameterControllerInterface)
    (Class|AudioParameterControllerInterface|SetTriggerParameter _audio "Trigger")))

(event Input|KeyboardEvents|Ä
  (params (Key :type Key%20Structure :default "None"))
  (bind _audio (Variables|Default|GetAudio))
  (:Pressed
    (Audio|Parameter|SetFloatParameter _audio "MIDI In" 64.0 :!class /Script/AudioExtensions.AudioParameterControllerInterface)
    (Class|AudioParameterControllerInterface|SetTriggerParameter _audio "Trigger")))

(event Input|KeyboardEvents|#
  (params (Key :type Key%20Structure :default "None"))
  (bind _audio (Variables|Default|GetAudio))
  (:Pressed
    (Audio|Parameter|SetFloatParameter _audio "MIDI In" 68.0 :!class /Script/AudioExtensions.AudioParameterControllerInterface)
    (Class|AudioParameterControllerInterface|SetTriggerParameter _audio "Trigger")))

(fn ConstructionScript)